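; BP_StorageCube is a storage crate that collects Ronk_Actor items of a single type, identified by each item's first actor tag.
; Hits on its Plane set the stored type from the first item, then count and destroy matching items.
; Mismatched or non-Ronk objects get an upward impulse and a Vineboom sound, while BP_JoeCharacter is ignored.
; Type, count and rejections are reported through debug prints.
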(event OnComponentHit(Plane)
  (params (HitComponent :type Primitive%20Component%20Object%20Reference) (OtherActor :type Actor%20Object%20Reference) (OtherComp :type Primitive%20Component%20Object%20Reference) (NormalImpulse :type Vector :default "0, 0, 0") (Hit :type Hit%20Result%20Structure%20%28by%20ref%29))
  (bind _tags (Variables|/Script/Engine.Actor|GetTags OtherActor))
  (bind _output (Utilities|Array|Get(acopy) _tags))
  (bind _returnvalue (Utilities|String|ToString(Name) _output))
  (if (== (Utilities|GetClass OtherActor) "/Game/_GENERATED/Joemama/Ronk/Ronk_Actor.Ronk_Actor_C")
    (if (Utilities|Enum|Equal(Enum) (Variables|Default|GetCurrentlyStored) "Nothing")
      (bind _output_get (Variables|Default|SetCurrentlyStored _returnvalue))
      (Development|PrintString _output_get)
      (bind _output_get_2 (Variables|Default|SetCurrentlyStoredCount (+ (Variables|Default|GetCurrentlyStoredCount) 1) :!label _label))
      (Actor|DestroyActor OtherActor)
      (Development|PrintString (Utilities|String|ToString(Integer) _output_get_2))
      (elif (Utilities|Enum|Equal(Enum) (Variables|Default|GetCurrentlyStored) _returnvalue)
        (bind _output_get_3 (Variables|Default|SetCurrentlyStored _returnvalue))
        (Development|PrintString _output_get_3)
        (goto _label)
        (else
          (Development|PrintString "Rejected, not what is in crate")
          (Physics|AddImpulse OtherComp "0.000000,0.000000,100.000000" "None" false :!label _label_2)
          (Audio|PlaySoundatLocation "/Game/_GENERATED/Zacchary/Objects/Props/Audio/vine-boom.vine-boom" (Transformation|GetActorLocation) "0, 0, 0" 0.5 1.0 0.0 0 0 0 0))))
    (elif (not (== (Utilities|GetClass OtherActor) "/Game/_GENERATED/Joemama/BP_JoeCharacter.BP_JoeCharacter_C"))
      (Development|PrintString "Rejected, not is not rank")
      (goto _label_2))))

(event EventBeginPlay)

(event Collision|EventActorBeginOverlap
  (params (OtherActor :type Actor%20Object%20Reference)))

(event EventTick
  (params (DeltaSeconds :type Float%20%28single-precision%29)))

(fn ConstructionScript)