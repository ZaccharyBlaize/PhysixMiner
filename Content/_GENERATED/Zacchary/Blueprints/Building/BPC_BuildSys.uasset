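; Player building component for BP_NewRonkChar that lets the player preview, rotate and place a build piece.
; While the toggled build mode is on, Tick line-traces from the follow camera and moves a non-colliding ghost plank mesh to the hit point.
; A DoOnce creates the ghost, then resets when build mode exits.
; Looping timers step preview rotation while rotate inputs are held, and placing spawns an actor at the preview transform.
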(event Custom|Preview%20Loop
  (bind _camera (Variables|Default|GetCamera))
  (bind _returnvalue (Transformation|GetWorldTransform _camera))
  ;[1 1 1] Trace Ghosts
  (bind (_outhit _returnvalue_2) (Collision|LineTraceByChannel (.location _returnvalue) (+ (.location _returnvalue) (* (Math|Vector|GetForwardVector (.rotation _returnvalue)) 7e+02)) "TraceTypeQuery1" false 0 "None"))
  (if _returnvalue_2
    (Utilities|FlowControl|Sequence
      (:then_0
        (Utilities|FlowControl|DoOnce false
          (:Completed
            (bind _returnvalue_3 (Game|AddComponentbyClass (Variables|Default|GetPlayerBp) "/Script/Engine.StaticMeshComponent" false (Variables|Default|GetBuildPreviewTransform)))
            (bind _output_get (Variables|Default|SetPreviewMesh _returnvalue_3))
            (Components|StaticMesh|SetStaticMesh _output_get "/Game/Crystal_cave/Meshes/Wood_props/SM_wood_planks_02.SM_wood_planks_02")
            (Rendering|Material|SetMaterial (Variables|Default|GetPreviewMesh) 0 "/Game/_GENERATED/Zacchary/Materials/M_BuildPreview.M_BuildPreview")
            (Collision|SetCollisionEnabled (Variables|Default|GetPreviewMesh) "NoCollision"))))
      (:then_1
        (bind _output_get_2 (Variables|Default|SetBuildPreviewTransform (Math|Transform|MakeTransform (.Location (Collision|BreakHitResult _outhit)) (Variables|Default|GetBuildPreviewRotation) "1.000000,1.000000,1.000000")))
        (Transformation|SetWorldTransform (Variables|Default|GetPreviewMesh) _output_get_2 false false)))))

(event Custom|Reset%20BuildMode
  ;[1 1 1] Trace Ghosts
  (Utilities|FlowControl|DoOnce false) ; enters at Reset
)

(event Custom|Rotate+
  ;[1 1 1] Rotate +
  (Variables|Default|SetBuildPreviewRotation (Math|Rotator|CombineRotators (.rotation (Variables|Default|GetBuildPreviewTransform)) "0.000000,5.000000,0.000000")))

(event Custom|Rotate-
  ;[1 1 1] Rotate -
  (Variables|Default|SetBuildPreviewRotation (Math|Rotator|CombineRotators (.rotation (Variables|Default|GetBuildPreviewTransform)) "0.000000,-5.000000,0.000000")))

(event Input|EnhancedActionEvents|EnhancedInputActionIA_Build
  (params (ActionValue :type Boolean) (ElapsedSeconds :type Float%20%28double-precision%29) (TriggeredSeconds :type Float%20%28double-precision%29) (InputAction :type Input%20Action%20Object%20Reference :default "/Game/_GENERATED/Zacchary/Blueprints/Char/Input/Actions/IA_Build.IA_Build"))
  ;[1 1 1] Control Build Mode
  (:Started
    (Utilities|FlowControl|FlipFlop
      (:A
        (Variables|Default|SetinBuildMode true))
      (:B
        (Variables|Default|SetinBuildMode false)
        (bind _previewmesh (Variables|Default|GetPreviewMesh)
          (:then
            (Components|StaticMesh|SetStaticMesh _previewmesh 0)
            (Variables|Default|SetPreviewMesh 0)
            (CallFunction|ResetBuildMode))
          (:else))))))

(event Input|EnhancedActionEvents|EnhancedInputActionIA_BuildPlace
  (params (ActionValue :type Boolean) (ElapsedSeconds :type Float%20%28double-precision%29) (TriggeredSeconds :type Float%20%28double-precision%29) (InputAction :type Input%20Action%20Object%20Reference :default "/Game/_GENERATED/Zacchary/Blueprints/Char/Input/Actions/IA_BuildPlace.IA_BuildPlace"))
  ;[1 1 1] Place
  (:Started
    (if (Variables|Default|GetinBuildMode)
      (Game|SpawnActorfromClass "/Game/_GENERATED/Zacchary/Blueprints/Building/BP_Build_Floor.BP_Build_Floor_C" (Variables|Default|GetBuildPreviewTransform) "AlwaysSpawn" "MultiplyWithRoot" 0 0))))

(event Input|EnhancedActionEvents|EnhancedInputActionIE_BuildRotate-
  (params (ActionValue :type Boolean) (ElapsedSeconds :type Float%20%28double-precision%29) (TriggeredSeconds :type Float%20%28double-precision%29) (InputAction :type Input%20Action%20Object%20Reference :default "/Game/_GENERATED/Zacchary/Blueprints/Char/Input/Actions/IE_BuildRotate-.IE_BuildRotate-"))
  ;[1 1 1] Rotate -
  (:Started
    (bind _returnvalue (Utilities|Time|SetTimerbyEvent (delegate Custom|Rotate-) 0.1 true))
    (Variables|Default|SetRotate-Loop _returnvalue))
  (:Canceled
    (Utilities|Time|ClearandInvalidateTimerbyHandle (Variables|Default|GetRotate-Loop) :!label _label)
    (Variables|Default|SetRotate-Loop ""))
  (:Completed
    (goto _label)))

(event Input|EnhancedActionEvents|EnhancedInputActionIE_BuildRotate+
  (params (ActionValue :type Boolean) (ElapsedSeconds :type Float%20%28double-precision%29) (TriggeredSeconds :type Float%20%28double-precision%29) (InputAction :type Input%20Action%20Object%20Reference :default "/Game/_GENERATED/Zacchary/Blueprints/Char/Input/Actions/IE_BuildRotate+.IE_BuildRotate+"))
  ;[1 1 1] Rotate +
  (:Started
    (bind _returnvalue (Utilities|Time|SetTimerbyEvent (delegate Custom|Rotate+) 0.1 true))
    (Variables|Default|SetRotate+Loop _returnvalue))
  (:Canceled
    (Utilities|Time|ClearandInvalidateTimerbyHandle (Variables|Default|GetRotate+Loop) :!label _label)
    (Variables|Default|SetRotate+Loop ""))
  (:Completed
    (goto _label)))

(event EventTick
  (params (DeltaSeconds :type Float%20%28single-precision%29))
  ;[1 1 1] Event Tick - Fire Preview
  (if (Variables|Default|GetinBuildMode)
    (CallFunction|PreviewLoop)))

(event EventBeginPlay
  ;[1 1 1] Init Raycast
  (bind _asbp_new_ronk_char (Utilities|Casting|CastToBP_NewRonkChar (Components|GetOwner)))
  (Variables|Default|SetPlayerBp _asbp_new_ronk_char)
  (Variables|Default|SetCamera (Variables|/Game/_GENERATED/Zacchary/Blueprints/Char/BP_NewRonkChar.BP_NewRonkChar_C|GetFollowCamera _asbp_new_ronk_char)))