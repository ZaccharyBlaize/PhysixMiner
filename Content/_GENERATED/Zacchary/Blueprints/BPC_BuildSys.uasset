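; BPC_BuildSys is a build-mode component for BP_NewRonkChar that previews a round table where the player's camera points.
; IA_Build toggles build mode; while active, Tick runs a short forward visibility trace from the follow camera.
; The first hit spawns a preview mesh with a build material via DoOnce, then each hit moves it to the impact location.
; Exiting clears the mesh without destroying its component and resets the DoOnce; nothing places objects.
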(event Custom|Preview%20Loop
  (bind _camera (Variables|Default|GetCamera))
  (bind _returnvalue (Transformation|GetWorldTransform _camera))
  (bind (_outhit _returnvalue_2) (Collision|LineTraceByChannel (.location _returnvalue) (+ (.location _returnvalue) (* (Math|Vector|GetForwardVector (.rotation _returnvalue)) 7e+02)) "TraceTypeQuery1" false 0 "None"))
  (if _returnvalue_2
    (Utilities|FlowControl|Sequence
      (:then_0
        (Utilities|FlowControl|DoOnce false
          (:Completed
            (bind _returnvalue_3 (Game|AddComponentbyClass (Variables|Default|GetPlayerBp) "/Script/Engine.StaticMeshComponent" false (Variables|Default|GetBuildPreviewTransform)))
            (bind _output_get (Variables|Default|SetPreviewMesh _returnvalue_3))
            (Components|StaticMesh|SetStaticMesh _output_get "/Game/StarterContent/Props/SM_TableRound.SM_TableRound")
            (Rendering|Material|SetMaterial (Variables|Default|GetPreviewMesh) 0 "/Game/_GENERATED/Zacchary/Materials/M_BuildPreview.M_BuildPreview"))))
      (:then_1
        (bind _output_get_2 (Variables|Default|SetBuildPreviewTransform (Math|Transform|MakeTransform (.Location (Collision|BreakHitResult _outhit)) "0, 0, 0" "1.000000,1.000000,1.000000")))
        (Transformation|SetWorldTransform (Variables|Default|GetPreviewMesh) _output_get_2 false false)))))

(event Custom|Reset%20BuildMode
  (Utilities|FlowControl|DoOnce false) ; enters at Reset
)

(event Input|EnhancedActionEvents|EnhancedInputActionIA_Build
  (params (ActionValue :type Boolean) (ElapsedSeconds :type Float%20%28double-precision%29) (TriggeredSeconds :type Float%20%28double-precision%29) (InputAction :type Input%20Action%20Object%20Reference :default "/Game/_GENERATED/Zacchary/Blueprints/Char/Input/Actions/IA_Build.IA_Build"))
  (:Started
    (Utilities|FlowControl|FlipFlop
      (:A
        (Variables|Default|SetinBuildMode true))
      (:B
        (Variables|Default|SetinBuildMode false)
        (Components|StaticMesh|SetStaticMesh (Variables|Default|GetPreviewMesh) 0)
        (Variables|Default|SetPreviewMesh 0)
        (CallFunction|ResetBuildMode)))))

(event EventTick
  (params (DeltaSeconds :type Float%20%28single-precision%29))
  (if (Variables|Default|GetinBuildMode)
    (CallFunction|PreviewLoop)))

(event EventBeginPlay
  (bind _asbp_new_ronk_char (Utilities|Casting|CastToBP_NewRonkChar (Components|GetOwner)))
  (Variables|Default|SetPlayerBp _asbp_new_ronk_char)
  (Variables|Default|SetCamera (Variables|/Game/_GENERATED/Zacchary/Blueprints/Char/BP_NewRonkChar.BP_NewRonkChar_C|GetFollowCamera _asbp_new_ronk_char)))