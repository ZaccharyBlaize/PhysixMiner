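; BpNewRonk is a rock actor that sets its appearance when play begins.
; It picks a random mesh from MeshIndex, then applies the material whose position in MaterialIndex matches RockAssignedType's position in the Materials array.
; DefineRockType holds unconnected logic for randomly choosing Gold, Iron or Stone and spawning a rock of that type, so it does nothing.
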(event EventBeginPlay
  (CallFunction|AssignStaticMesh)
  (CallFunction|AssignMaterials))

(event Collision|EventActorBeginOverlap
  (params (OtherActor :type Actor%20Object%20Reference)))

(event EventTick
  (params (DeltaSeconds :type Float%20%28single-precision%29)))

(fn ConstructionScript)

(fn AssignMaterials
  (Rendering|Material|SetMaterial (Variables|Default|GetStaticMesh) 0 (Utilities|Array|Get(acopy) (Variables|Default|GetMaterialIndex) (Utilities|Array|FindItem (Variables|Default|GetMaterials) (Variables|Default|GetRockAssignedType)))))

(fn AssignStaticMesh
  (Components|StaticMesh|SetStaticMesh (Variables|Default|GetStaticMesh) (Utilities|Array|Get(acopy) (Variables|Default|GetMeshIndex) (Math|Random|RandomInteger 4))))

(fn DefineRockType)