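; Spawner actor that launches pickups: clicking its Node component spawns a Ronk at the Arrow's transform and pushes it along world +X.
; SpawnRandomObject makes a weighted random pick of stone (most likely), iron or gold (rarest), spawns it at a jittered position above the actor and applies a random upward-biased impulse.
; Nothing in this Blueprint calls SpawnRandomObject; the click handler only spawns Ronk.
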(event OnClicked(Node)
  (params (TouchedComponent :type Primitive%20Component%20Object%20Reference) (ButtonPressed :type Key%20Structure :default "None"))
  (bind _returnvalue (Game|SpawnActorfromClass "/Game/_GENERATED/Joe/joerock/Ronk.Ronk_C" (Transformation|GetWorldTransform (Variables|Default|GetArrow)) "Undefined" "MultiplyWithRoot" 0 0))
  (Physics|AddImpulse (Variables|/Game/_GENERATED/Joe/joerock/Ronk.Ronk_C|GetStaticMesh _returnvalue) "3000.000000,0.000000,0.000000" "None" false))

(event EventBeginPlay)

(event Collision|EventActorBeginOverlap
  (params (OtherActor :type Actor%20Object%20Reference)))

(event EventTick
  (params (DeltaSeconds :type Float%20%28single-precision%29)))

(fn ConstructionScript)

(fn SpawnRandomObject
  (bind _returnvalue (Transformation|GetActorTransform))
  (bind _returnvalue_2 (Math|Random|RandomFloatinRange 2e+01 2e+02))
  (bind _returnvalue_3 (Math|Random|RandomFloatinRange -1e+01 1e+01))
  (bind _returnvalue_4 (Math|Random|RandomFloatinRange 8e+01 1e+02))
  (bind _returnvalue_5 (Math|Random|RandomFloatinRange -1e+01 1e+01))
  (bind _returnvalue_6 (Math|Random|RandomFloatinRange -1e+02 1e+02))
  (bind _returnvalue_7 (Math|Random|RandomFloatinRange -1e+02 1e+02))
  (bind _returnvalue_8 (+ (.z (.location _returnvalue)) _returnvalue_2))
  (bind _returnvalue_9 (+ (.x (.location _returnvalue)) _returnvalue_3))
  (bind _returnvalue_10 (+ (.y (.location _returnvalue)) _returnvalue_5))
  (bind _output_get (Variables|Default|SetRandomIndex (Math|Random|RandomIntegerinRange 0 10)))
  (if (>= _output_get 3)
    (bind _returnvalue_11 (Game|SpawnActorfromClass "/Game/_GENERATED/Zacchary/Blueprints/BpStone.BpStone_C" (Math|Transform|MakeTransform (Math|Vector|MakeVector _returnvalue_9 _returnvalue_10 _returnvalue_8) (.rotation _returnvalue) (.scale _returnvalue)) "AdjustIfPossibleButAlwaysSpawn" "MultiplyWithRoot" 0 0))
    (Physics|AddImpulse (Variables|/Script/Engine.StaticMeshActor|GetStaticMeshComponent _returnvalue_11) (Math|Vector|MakeVector _returnvalue_7 _returnvalue_6 _returnvalue_4) "None" false)
    (elif (>= _output_get 1)
      (bind _returnvalue_12 (Game|SpawnActorfromClass "/Game/_GENERATED/Zacchary/Blueprints/BpIron.BpIron_C" (Math|Transform|MakeTransform (Math|Vector|MakeVector _returnvalue_9 _returnvalue_10 _returnvalue_8) (.rotation _returnvalue) (.scale _returnvalue)) "AdjustIfPossibleButAlwaysSpawn" "MultiplyWithRoot" 0 0))
      (Physics|AddImpulse (Variables|/Script/Engine.StaticMeshActor|GetStaticMeshComponent _returnvalue_12) (Math|Vector|MakeVector _returnvalue_7 _returnvalue_6 _returnvalue_4) "None" false)
      (else
        (bind _returnvalue_13 (Game|SpawnActorfromClass "/Game/_GENERATED/Zacchary/Blueprints/BpGold.BpGold_C" (Math|Transform|MakeTransform (Math|Vector|MakeVector _returnvalue_9 _returnvalue_10 _returnvalue_8) (.rotation _returnvalue) (.scale _returnvalue)) "AdjustIfPossibleButAlwaysSpawn" "MultiplyWithRoot" 0 0))
        (Physics|AddImpulse (Variables|/Script/Engine.StaticMeshActor|GetStaticMeshComponent _returnvalue_13) (Math|Vector|MakeVector _returnvalue_7 _returnvalue_6 _returnvalue_4) "None" false)))))