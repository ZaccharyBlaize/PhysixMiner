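; Storage crate actor that stores BpNewRonk rocks of a single type and dispenses them on demand.
; Hits on the input plane absorb matching rocks and update count and type text, while rejects other than the player are flung away randomly.
; Tick polls the player's hitscan interface for button hits, toggling output that respawns rocks through a one-second Delay until empty, with a red/green status light.
; Left/right filter buttons only print; their filter-changing logic is disconnected.
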(event OnComponentHit(InputPlane)
  (params (HitComponent :type Primitive%20Component%20Object%20Reference) (OtherActor :type Actor%20Object%20Reference) (OtherComp :type Primitive%20Component%20Object%20Reference) (NormalImpulse :type Vector :default "0, 0, 0") (Hit :type Hit%20Result%20Structure%20%28by%20ref%29))
  ;[1 1 1] What's going Into the Box logic
  (bind _asbp_new_ronk (Utilities|Casting|CastToBpNewRonk OtherActor))
  (if (== (Utilities|GetClass OtherActor) "/Game/_GENERATED/Zacchary/Blueprints/BpNewRonk.BpNewRonk_C")
    (if (Utilities|Enum|Equal(Enum) (Variables|Default|GetCurrentlyStored) "Nothing")
      (bind _output_get (Variables|Default|SetCurrentlyStored (Variables|/Game/_GENERATED/Zacchary/Blueprints/BpNewRonk.BpNewRonk_C|GetRockAssignedType _asbp_new_ronk)))
      (Development|PrintString _output_get)
      (bind _output_get_2 (Variables|Default|SetCurrentlyStoredCount (+ (Variables|Default|GetCurrentlyStoredCount) 1) :!label _label))
      (Actor|DestroyActor OtherActor)
      (Rendering|Components|TextRender|SetText (Variables|Default|GetCount) (Utilities|Text|ToText(String) (Utilities|String|ToString(Integer) _output_get_2)))
      (Rendering|Components|TextRender|SetText (Variables|Default|GetStored) (Utilities|Text|ToText(String) (Variables|Default|GetCurrentlyStored)))
      (Development|PrintString (Utilities|String|ToString(Integer) _output_get_2))
      (elif (Utilities|Enum|Equal(Enum) (Variables|Default|GetCurrentlyStored) (Variables|/Game/_GENERATED/Zacchary/Blueprints/BpNewRonk.BpNewRonk_C|GetRockAssignedType _asbp_new_ronk))
        (bind _output_get_3 (Variables|Default|SetCurrentlyStored (Variables|/Game/_GENERATED/Zacchary/Blueprints/BpNewRonk.BpNewRonk_C|GetRockAssignedType _asbp_new_ronk)))
        (Development|PrintString _output_get_3)
        (goto _label)
        (else
          (Development|PrintString "Rejected, not what is in crate")
          (Class|PrimitiveComponent|AddVelocityChangeImpulseatLocation OtherComp (Math|Vector|MakeVector (Math|Conversions|ToFloat(Integer) (Math|Random|RandomIntegerinRange -300 300)) (Math|Conversions|ToFloat(Integer) (Math|Random|RandomIntegerinRange -300 300)) (Math|Conversions|ToFloat(Integer) (Math|Random|RandomIntegerinRange 250 400))) (Transformation|GetActorLocation) "None" :!label _label_2))))
    (elif (not (== (Utilities|GetClass OtherActor) "/Game/_GENERATED/Joemama/BP_JoeCharacter.BP_JoeCharacter_C"))
      (Development|PrintString "Rejected, not suitable for crate")
      (goto _label_2))))

(event EventBeginPlay
  ;[1 1 1] Set on Init to Nothing Nothing
  (Rendering|Components|TextRender|SetText (Variables|Default|GetCount) (Utilities|Text|ToText(String) (Utilities|String|ToString(Integer) (Variables|Default|GetCurrentlyStoredCount))))
  (Rendering|Components|TextRender|SetText (Variables|Default|GetStored) (Utilities|Text|ToText(String) (Variables|Default|GetCurrentlyStored)))
  (Variables|Default|SetFilterIndex 0)
  (bind _returnvalue (Actor|GetActorOfClass "/Game/_GENERATED/Joemama/Ronk/Ronk_Actor.Ronk_Actor_C"))
  (for _array_element (Variables|/Script/Engine.Actor|GetTags _returnvalue)
    (bind _output_get (Variables|Default|SetStringArrayFilter (Utilities|Array|MakeArray (.OutTagValue (Class|AssetRegistryHelpers|GetTagValue (Utilities|Struct|MakeAssetData) _array_element)))))
    (for _array_element_2 _output_get
      (Development|PrintString _array_element_2))))

(event Collision|EventActorBeginOverlap
  (params (OtherActor :type Actor%20Object%20Reference)))

(event EventTick
  (params (DeltaSeconds :type Float%20%28single-precision%29))
  (bind _out (Variables|Default|GetOut))
  (bind _returnvalue (Transformation|GetWorldTransform _out))
  (CallFunction|SetLightOff)
  (Utilities|FlowControl|Sequence
    (:then_0
      ;[1 1 1] Spawn Ronks
      (if (== (Variables|Default|GetStorageStatus) 1)
        (Utilities|FlowControl|Delay 1.0)
        (Game|SpawnActorfromClass "/Game/_GENERATED/Zacchary/Blueprints/BpNewRonk.BpNewRonk_C" (Math|Transform|MakeTransform (Math|Vector|MakeVector (.x (.location _returnvalue)) (+ (.y (.location _returnvalue)) 1e+01) (+ (.z (.location _returnvalue)) 3e+01)) "0, 0, 0" "1.000000,1.000000,1.000000") "Undefined" "MultiplyWithRoot" 0 (Variables|Default|GetCurrentlyStored) "0.000000,0.000000,0.000000|0.000000,0.000000,-0.000000|1.000000,1.000000,1.000000" 0)
        (bind _result (Math|Integer|DecrementInt (Variables|Default|GetCurrentlyStoredCount))
          (:%20%20
            (Rendering|Components|TextRender|SetText (Variables|Default|GetCount) (Utilities|Text|ToText(Integer) _result))
            (if (== _result 0)
              (Variables|Default|SetStorageStatus 0)
              (Rendering|Material|SetMaterial (Variables|Default|GetStorage%20Light) 0 "/Game/Crystal_cave/Materials/MI_ore_Red.MI_ore_Red")
              (if (not (Variables|Default|GetManuallySet))
                (bind _output_get (Variables|Default|SetCurrentlyStored "Nothing"))
                (Rendering|Components|TextRender|SetText (Variables|Default|GetStored) (Utilities|Text|ToText(String) _output_get))))))))
    (:then_1
      ;[1 1 1] Define What has been Hit By Hitscan
      (bind _hit_result (Class|JoeCharInterface|IFGetHitscan(Message) (Game|GetPlayerCharacter 0)))
      (if (== (Variables|Default|GetStorage%20Button) (.HitComponent (Collision|BreakHitResult _hit_result)))
        ;[1 1 1] Hit Button = If not outputting and Stored >= 1 then swap to outputting
        (if (== (Variables|Default|GetStorageStatus) 0)
          (if (>= (Variables|Default|GetCurrentlyStoredCount) 1)
            (Variables|Default|SetStorageStatus 1)
            (Rendering|Material|SetMaterial (Variables|Default|GetStorage%20Light) 0 "/Game/Crystal_cave/Materials/MI_ore_Green.MI_ore_Green"))
          (else
            (Variables|Default|SetStorageStatus 0)))
        (elif (== (Variables|Default|GetButton%20Right) (.HitComponent (Collision|BreakHitResult _hit_result)))
          (Development|PrintString "Right")
          (elif (== (Variables|Default|GetButton%20Left) (.HitComponent (Collision|BreakHitResult _hit_result)))
            (Development|PrintString "Left")))))))

(fn ConstructionScript)

(fn SetLightOff
  (if (== (Variables|Default|GetStorageStatus) 0)
    (Variables|Default|SetStorageStatus 0)
    (Rendering|Material|SetMaterial (Variables|Default|GetStorage%20Light) 0 "/Game/Crystal_cave/Materials/MI_ore_Red.MI_ore_Red")
    (return)))

(fn IFGetHitscan
  (return ""))