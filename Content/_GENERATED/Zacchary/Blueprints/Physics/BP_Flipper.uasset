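; BP_Flipper is an actor whose mesh continuously flips back and forth on its own.
; On BeginPlay it stores the mesh's initial rotation, derives a target offset by a quarter turn in roll with pitch and yaw zeroed, and starts flipping.
; A FlipFlop alternately plays and reverses a timeline that lerps between both rotations and, when finished, triggers the next flip after a short delay.
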(event Custom|Flip
  (params (Debug1%20 :type String))
  (Utilities|FlowControl|FlipFlop
    (:A
      (Variables|Default|SetIsFlipped true)
      (bind _rotation_value (Timeline|Rotation%20Timeline Play)
        (:Update
          (Transformation|SetRelativeRotation (Variables|Default|GetFlipperMesh) (Math|Rotator|Lerp(Rotator) (Variables|Default|GetInitial%20Rotation) (Variables|Default|GetTarget%20Rotation) _rotation_value) false false))
        (:Finished
          (Utilities|FlowControl|Delay 1.0)
          (CallFunction|Flip "Flip Event Called"))))
    (:B
      (Variables|Default|SetIsFlipped false)
      (Timeline|Rotation%20Timeline Reverse))))

(event EventBeginPlay
  (bind _output_get (Variables|Default|SetInitial%20Rotation (Variables|/Script/Engine.SceneComponent|GetRelativeRotation (Variables|Default|GetFlipperMesh))))
  (Variables|Default|SetTarget%20Rotation (Math|Rotator|MakeRotator (+ (.roll _output_get) -9e+01) 0.0 0.0))
  (CallFunction|Flip "Flip Event Called"))

(fn ConstructionScript)